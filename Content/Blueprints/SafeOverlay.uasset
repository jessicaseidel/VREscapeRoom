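; SafeOverlay is a keypad overlay for unlocking a safe with a hardcoded four-digit code.
; The show event stores the Safe and makes the buttons, text and mesh visible and queryable.
; CodeSafe builds the code through a branch chain per pressed button, resetting on out-of-order correct digits and ignoring other buttons.
; Ready with the full code hides the overlay, disables its collision and unlocks the Safe, with feedback via PrintString.
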(event Custom|show
  (params (NewParam :type Safe%20Object%20Reference))
  (bind _safeoverlay_text_018 (Variables|Default|Getsafeoverlay_Text_018))
  (bind _staticmesh (Variables|Default|GetStaticMesh))
  (bind _safeoverlay_text_010 (Variables|Default|Getsafeoverlay_Text_010))
  (bind _safeoverlay_text_011 (Variables|Default|Getsafeoverlay_Text_011))
  (bind _safeoverlay_text_012 (Variables|Default|Getsafeoverlay_Text_012))
  (bind _safeoverlay_text_014 (Variables|Default|Getsafeoverlay_Text_014))
  (bind _safeoverlay_text_013 (Variables|Default|Getsafeoverlay_Text_013))
  (bind _safeoverlay_text_015 (Variables|Default|Getsafeoverlay_Text_015))
  (bind _safeoverlay_text_016 (Variables|Default|Getsafeoverlay_Text_016))
  (bind _safeoverlay_text_017 (Variables|Default|Getsafeoverlay_Text_017))
  (bind _safeoverlay_text_019 (Variables|Default|Getsafeoverlay_Text_019))
  (bind _button1 (Variables|Default|GetButton1))
  (bind _button3 (Variables|Default|GetButton3))
  (bind _button2 (Variables|Default|GetButton2))
  (bind _button4 (Variables|Default|GetButton4))
  (bind _button6 (Variables|Default|GetButton6))
  (bind _button7 (Variables|Default|GetButton7))
  (bind _button9 (Variables|Default|GetButton9))
  (bind _button5 (Variables|Default|GetButton5))
  (bind _button8 (Variables|Default|GetButton8))
  (bind _buttonexit (Variables|Default|GetButtonExit))
  (bind _button0 (Variables|Default|GetButton0))
  (bind _buttonready (Variables|Default|GetButtonReady))
  (bind _array (Utilities|Array|MakeArray _safeoverlay_text_010 _safeoverlay_text_011 _safeoverlay_text_012 _safeoverlay_text_013 _safeoverlay_text_014 _safeoverlay_text_015 _safeoverlay_text_016 _safeoverlay_text_017 _safeoverlay_text_019 _button1 _button2 _button3 _button4 _button5 _button6 _button7 _button8 _button9 _buttonexit _button0 _buttonready _staticmesh _safeoverlay_text_018))
  (Variables|Default|SetSafe NewParam)
  (for _array_element _array
    (Rendering|SetVisibility _array_element true false)
    (for _array_element_2 _array
      (Collision|SetCollisionEnabled _array_element_2 "QueryOnly"))))

(event EventBeginPlay)

(event Collision|EventActorBeginOverlap
  (params (OtherActor :type Actor%20Object%20Reference)))

(event EventTick
  (params (DeltaSeconds :type Float%20%28single-precision%29)))

(fn ConstructionScript)

(fn CodeSafe
  (params (NewParam1 :type Object%20Object%20Reference))
  (Development|PrintString (Utilities|String|ToString(Object) NewParam1))
  (if (== (Variables|Default|GetButton9) NewParam1)
    (if (Utilities|Enum|Equal(Enum) (Variables|Default|GetCode) (Variables|Default|Get****))
      (Variables|Default|SetCode "9")
      (Development|PrintString " 
 
 
 
 
 
 
 
 
 
 
 
 
 
 
 
 
 
 
                                                                      9")
      (else
        (Variables|Default|SetCode "****" :!label _label)
        (Development|PrintString " 
 
 
 
 
 
 
 
 
 
 
 
 
 
 
 
 
 
 
 
 
 
 
 
 
 
 
 
 
 
 
 
 
 
 
 
 
                                                    ERROR" true true "(R=0.553820,G=0.008653,B=0.030415,A=1.000000)")))
    (elif (== NewParam1 (Variables|Default|GetButton1))
      (if (Utilities|Enum|Equal(Enum) (Variables|Default|GetCode) (Variables|Default|Get9))
        (Variables|Default|SetCode "91")
        (Development|PrintString " 
 
 
 
 
 
 
 
 
 
 
 
 
 
 
 
 
 
 
                                                                      91")
        (else
          (goto _label)))
      (elif (== NewParam1 (Variables|Default|GetButton6))
        (if (Utilities|Enum|Equal(Enum) (Variables|Default|GetCode) (Variables|Default|Get91))
          (Variables|Default|SetCode "916")
          (Development|PrintString " 
 
 
 
 
 
 
 
 
 
 
 
 
 
 
 
 
 
 
                                                                      916")
          (else
            (goto _label)))
        (elif (== NewParam1 (Variables|Default|GetButton2))
          (if (Utilities|Enum|Equal(Enum) (Variables|Default|GetCode) (Variables|Default|Get916))
            (Variables|Default|SetCode "9162")
            (Development|PrintString " 
 
 
 
 
 
 
 
 
 
 
 
 
 
 
 
 
 
 
                                                                      9162")
            (else
              (goto _label)))
          (elif (== NewParam1 (Variables|Default|GetButtonReady))
            (if (Utilities|Enum|Equal(Enum) (Variables|Default|GetCode) (Variables|Default|Get9162))
              (Development|PrintString " 
 
 
 
 
 
 
 
 
 
 
 
 
 
 
 
 
 
 
 
 
 
 
 
 
 
 
 
 
 
 
 
 
 
 
 
 
                                                    OPEN" true true "(R=0.086674,G=0.553820,B=0.066147,A=1.000000)")
              (for _array_element (Utilities|Array|MakeArray (Variables|Default|Getsafeoverlay_Text_010) (Variables|Default|Getsafeoverlay_Text_011) (Variables|Default|Getsafeoverlay_Text_012) (Variables|Default|Getsafeoverlay_Text_013) (Variables|Default|Getsafeoverlay_Text_014) (Variables|Default|Getsafeoverlay_Text_015) (Variables|Default|Getsafeoverlay_Text_016) (Variables|Default|Getsafeoverlay_Text_017) (Variables|Default|Getsafeoverlay_Text_019) (Variables|Default|GetButton1) (Variables|Default|GetButton2) (Variables|Default|GetButton3) (Variables|Default|GetButton4) (Variables|Default|GetButton5) (Variables|Default|GetButton6) (Variables|Default|GetButton7) (Variables|Default|GetButton8) (Variables|Default|GetButton9) (Variables|Default|GetButtonExit) (Variables|Default|GetButton0) (Variables|Default|GetButtonReady) (Variables|Default|GetStaticMesh) (Variables|Default|Getsafeoverlay_Text_018))
                (Rendering|SetVisibility _array_element false false)
                (Collision|SetCollisionEnabled _array_element "NoCollision"))
              (bind _assafe (Utilities|Casting|CastToSafe (Variables|Default|GetSafe)))
              (Variables|/Game/Blueprints/Safe.Safe_C|SetLocked _assafe false)
              (Development|PrintString " 
 
 
 
 
 
 
 
 
 
 
 
 
 
 
                                                               fzck")
              (else
                (Development|PrintString "doof")
                (goto _label)))))))))