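; Interactable drawer Blueprint (Schublade) that toggles between open and closed whenever its Pickup event fires.
; A Move flag selects whether the mesh slides or rotates, so it also covers hinged objects.
; Two timelines scale configurable per-axis offsets or angles by a blend value, playing forward to open and reversing to close.
; The construction script applies a uniform mesh scale and an optional mesh override.
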(event EventPickup
  (params (AttachTo :type Scene%20Component%20Object%20Reference))
  (if (Variables|Default|GetMove)
    (if (Variables|Default|GetClosed)
      (Variables|Default|SetClosed false)
      (bind _blend (Timeline|BlendOpenClose PlayFromStart)
        (:Update
          (Transformation|SetRelativeLocation (Variables|Components|GetStaticMesh) (Math|Vector|MakeVector (* _blend (Variables|Default|GetMoveX)) (* _blend (Variables|Default|GetMoveY)) (* _blend (Variables|Default|GetMoveZ))) false false)))
      (else
        (Variables|Default|SetClosed true)
        (Timeline|BlendOpenClose ReverseFromEnd)))
    (elif (Variables|Default|GetClosed)
      (Variables|Default|SetClosed false)
      (bind _blend_2 (Timeline|BlendRotate PlayFromStart)
        (:Update
          (Transformation|SetRelativeRotation (Variables|Components|GetStaticMesh) (Math|Rotator|MakeRotator (* _blend_2 (Variables|Default|GetRotateX)) (* _blend_2 (Variables|Default|GetRotateY)) (* _blend_2 (Variables|Default|GetRotateZ))) false false)))
      (else
        (Variables|Default|SetClosed true)
        (Timeline|BlendRotate ReverseFromEnd)))))

(fn ConstructionScript
  (bind _meshscale (Variables|Default|GetMeshScale))
  (bind _objectmesh (Variables|Default|GetObjectMesh))
  ;[1 1 1] Set Mesh Scale
  (Transformation|SetRelativeScale3D (Variables|Components|GetStaticMesh) (Math|Vector|MakeVector _meshscale _meshscale _meshscale))
  ;[1 1 1] Allow Mesh Override
  (if (!= _objectmesh 0)
    (Components|StaticMesh|SetStaticMesh (Variables|Components|GetStaticMesh) _objectmesh)))