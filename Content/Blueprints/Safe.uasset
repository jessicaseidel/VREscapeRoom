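; An interactable safe that stays shut while locked and otherwise toggles open and closed when Pickup fires.
; While locked, it prints a message and shows the SafeOverlay widget once, passing itself in, guarded by a visibility flag.
; When unlocked, the Move flag selects sliding the static mesh or rotating the Origin component.
; Timelines scale configurable per-axis amounts, playing forward to open and in reverse to close.
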(event EventPickup
  (params (AttachTo :type Scene%20Component%20Object%20Reference))
  (if (Variables|Default|GetLocked)
    (Development|PrintString " 
 
 
 
 
 
 
 
 
 
 
 
 
 
 
 
                                                                            LOCKED")
    ;[1 1 1] interact (show overlay)
    (if (not (Variables|Default|GetOverlayVisible))
      (Variables|Default|SetOverlayVisible true)
      (bind _assafe_overlay (Utilities|Casting|CastToSafeOverlay (Variables|Default|GetOverlay)))
      (Default|Show _assafe_overlay self))
    (else
      ;[1 1 1] move/rotate
      (if (Variables|Default|GetMove)
        (if (Variables|Default|GetClosed)
          (Variables|Default|SetClosed false)
          (bind _blend (Timeline|BlendOpenClose PlayFromStart)
            (:Update
              (Transformation|SetRelativeLocation (Variables|Components|GetStaticMesh) (Math|Vector|MakeVector (* _blend (Variables|Default|GetMoveX)) (* _blend (Variables|Default|GetMoveY)) (* _blend (Variables|Default|GetMoveZ))) false false)))
          (else
            (Variables|Default|SetClosed true)
            (Timeline|BlendOpenClose ReverseFromEnd)))
        (elif (Variables|Default|GetClosed)
          (Variables|Default|SetClosed false)
          (bind _blend_2 (Timeline|BlendRotate PlayFromStart)
            (:Update
              (Transformation|SetRelativeRotation (Variables|Default|GetOrigin) (Math|Rotator|MakeRotator (* _blend_2 (Variables|Default|GetRotateX)) (* _blend_2 (Variables|Default|GetRotateY)) (* _blend_2 (Variables|Default|GetRotateZ))) false false)))
          (else
            (Variables|Default|SetClosed true)
            (Timeline|BlendRotate ReverseFromEnd)))))))

(fn ConstructionScript)