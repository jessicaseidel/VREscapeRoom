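; LightSwitch is a Blueprint that turns a group of lights on and off when its Pickup event fires.
; The event checks the LightOn flag, then loops over the Light array to set each light component's intensity to zero or a fixed brightness.
; LightOn is updated inside each loop, so it changes only when the array has entries.
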(event EventBeginPlay)

(event Collision|EventActorBeginOverlap
  (params (OtherActor :type Actor%20Object%20Reference)))

(event EventTick
  (params (DeltaSeconds :type Float%20%28single-precision%29)))

(event EventPickup
  (params (AttachTo :type Scene%20Component%20Object%20Reference))
  (if (Variables|Default|GetLightOn)
    (for _array_element (Variables|Default|GetLight)
      (Rendering|Components|Light|SetIntensity (Variables|/Script/Engine.Light|GetLightComponent _array_element) 0.0)
      (Variables|Default|SetLightOn false))
    (else
      (for _array_element_2 (Variables|Default|GetLight)
        (Rendering|Components|Light|SetIntensity (Variables|/Script/Engine.Light|GetLightComponent _array_element_2) 2e+03)
        (Variables|Default|SetLightOn true)))))

(fn ConstructionScript)